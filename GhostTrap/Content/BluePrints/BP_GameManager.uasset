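; Game manager Blueprint that shows the number of key collectibles left in a HUD counter widget.
; BeginPlay creates the counter widget, writes the cached PreviousAmount and adds it to the viewport.
; Tick polls TotalKeyCollectibles, using SetScore for the first sync, then refreshes on changes by re-running the text and AddToViewport steps.
; Tick ignores a total of zero, so the display never updates to zero from there.
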(event `self.ReceiveBeginPlay`
  (bind _returnvalue (`|CreateWidget` "/Game/BluePrints/BP_CollectCounterWidget.BP_CollectCounterWidget_C"))
  (`TextBlock.SetText` (`/Game/BluePrints/BP_CollectCounterWidget.KeyCollectiblesLeft` _returnvalue) (`KismetTextLibrary.Conv_IntToText` (stale `self.ReceiveTick` _output_get)) :!label _label)
  (`UserWidget.AddToViewport` _returnvalue 0))

(event `self.ReceiveTick`
  (params (DeltaSeconds :type "Float (single-precision)"))
  (bind _totalkeycollectibles (`self.totalKeyCollectibles`))
  (if (!= (`self.totalKeyCollectibles`) 0)
    (if (`self.SetScore`)
      (if (!= _totalkeycollectibles (`self.previousAmount`))
        (set `self.previousAmount` (`self.totalKeyCollectibles`))
        (goto _label))
      (else
        (bind _output_get (set `self.previousAmount` _totalkeycollectibles))
        (set `self.SetScore` true)
        (goto _label)))))

(fn `UserConstructionScript`)